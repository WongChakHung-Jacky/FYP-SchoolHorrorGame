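; BP_Item is an interactable world item that the player can either inspect or pick up into the inventory.
; The construction script applies the Item struct's mesh and scale and sets up a sphere that shows a widget icon on player overlap, with separate focus highlighting.
; OnInteract either spawns a far-off BP_InspectItem to present the item or calls AddToInventory, optionally notifying tagged BP_objective actors once.
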(event `self.interaction_icon_show_range.OnComponentBeginOverlap`
  (params (OverlappedComponent :type "PrimitiveComponent Object Reference") (OtherActor :type "Actor Object Reference") (OtherComp :type "PrimitiveComponent Object Reference") (OtherBodyIndex :type Integer) (bFromSweep :type Boolean) (SweepResult :type "HitResult Structure (by ref)"))
  (if (== OtherActor (`GameplayStatics.GetPlayerCharacter` 0))
    (`/Game/SchoolHorrorGame/Blueprints/UI/W_Interaction_icon.Show/Hide Interact Icon` (`self.Interact_icon_widget_Ref`) true)))

(event `self.interaction_icon_show_range.OnComponentEndOverlap`
  (params (OverlappedComponent :type "PrimitiveComponent Object Reference") (OtherActor :type "Actor Object Reference") (OtherComp :type "PrimitiveComponent Object Reference") (OtherBodyIndex :type Integer))
  (if (== (`GameplayStatics.GetPlayerCharacter` 0) OtherActor)
    (`/Game/SchoolHorrorGame/Blueprints/UI/W_Interaction_icon.Show/Hide Interact Icon` (`self.Interact_icon_widget_Ref`) false)))

(event `/Game/SchoolHorrorGame/Blueprints/Interfaces/Interactable.Set_foucs`
  (params (Focus :type Boolean))
  (`/Game/SchoolHorrorGame/Blueprints/UI/W_Interaction_icon.Set_Focus` (`self.Interact_icon_widget_Ref`) Focus))

(event `self.ReceiveBeginPlay`
  (`|ExecutionSequence`
    (:`then_0`
      (`self.Beginplay_Get_Refs`))
    (:`then_1`
      (bind _asbp_player_character (cast `/Game/SchoolHorrorGame/Blueprints/BP_Player_Character` (`GameplayStatics.GetPlayerCharacter` 0)))
      (set `self.BP Player Ref` _asbp_player_character))))

(event `/Game/SchoolHorrorGame/InventorySystem/Blueprints/interactinterface.OnInteract`
  (params (Character :type "/Game/SchoolHorrorGame/Blueprints/BP_Player_Character Object Reference"))
  (bind (_itemname _itemstackable_ _itemamount _itemimage _itemmesh _iteminventory_ _itemdescription) (break `/Game/SchoolHorrorGame/InventorySystem/Blueprints/S_ItemStructure` (`self.Item`)))
  (if (`self.Inspect?`)
    (bind _returnvalue (`|SpawnActorFromClass` "/Game/SchoolHorrorGame/InventorySystem/Blueprints/Inspect/BP_InspectItem.BP_InspectItem_C" (`KismetMathLibrary.MakeTransform` (100000000.0 0.0 0.0)) "Undefined" "MultiplyWithRoot" null null))
    (`/Game/SchoolHorrorGame/InventorySystem/Blueprints/Inspect/BP_InspectItem.Set Inspect rotation` _returnvalue (`self.Item Inspection Rotation`))
    (`/Game/SchoolHorrorGame/InventorySystem/Blueprints/Inspect/BP_InspectItem.Set Inspect Scale` _returnvalue (`self.Item Inspection Scale`))
    (message `/Game/SchoolHorrorGame/InventorySystem/Blueprints/interactinterface.Inspect` _returnvalue Character _itemmesh _itemname _itemdescription)
    (if (`self.do objective`)
      (`/Engine/EditorBlueprintResources/StandardMacros.DoOnce` false
        (:`Completed`
          (bind _outactors (`GameplayStatics.GetAllActorsOfClassWithTag` "/Game/SchoolHorrorGame/InventorySystem/Blueprints/objective/BP_objective.BP_objective_C" (`self.Tag`)))
          (`/Game/SchoolHorrorGame/InventorySystem/Blueprints/objective/BP_objective.item objective` _outactors))))
    (else
      (`/Game/SchoolHorrorGame/InventorySystem/Blueprints/BPC_InventoryComponent.Add To Inventory` (`/Game/SchoolHorrorGame/Blueprints/BP_Player_Character.BP_InventoryComponent` Character) self)
      (if (`self.do objective`)
        (`/Engine/EditorBlueprintResources/StandardMacros.DoOnce` false
          (:`Completed`
            (bind _outactors_2 (`GameplayStatics.GetAllActorsOfClassWithTag` "/Game/SchoolHorrorGame/InventorySystem/Blueprints/objective/BP_objective.BP_objective_C" (`self.Tag`)))
            (`/Game/SchoolHorrorGame/InventorySystem/Blueprints/objective/BP_objective.item objective` _outactors_2)))))))

(fn `Beginplay_Get_Refs`
  (bind _asw_interaction_icon (cast `/Game/SchoolHorrorGame/Blueprints/UI/W_Interaction_icon` (`WidgetComponent.GetWidget` (`self.Interact_icon`))))
  (set `self.Interact_icon_widget_Ref` _asw_interaction_icon))

(fn `Get_Details`
  (returns (Result :type Boolean) (`Interaction text` :type Text))
  (return (`self.Can_intertact_variable`) (`.ItemName_17_2BD394214593178F12D7ABA528F32536` (break `/Game/SchoolHorrorGame/InventorySystem/Blueprints/S_ItemStructure` (`self.Item`)))))

(fn `UserConstructionScript`
  (bind _staticmesh (`self.StaticMesh`))
  (bind _interaction_icon_show_range (`self.interaction_icon_show_range`))
  (`|ExecutionSequence`
    (:`then_0`
      (`StaticMeshComponent.SetStaticMesh` _staticmesh (`.ItemMesh_27_A7B7E6A645C0C9F741243798C499B5C3` (break `/Game/SchoolHorrorGame/InventorySystem/Blueprints/S_ItemStructure` (`self.Item`))))
      (`SceneComponent.K2_SetWorldTransform` _staticmesh (`KismetMathLibrary.MakeTransform` (`SceneComponent.K2_GetComponentLocation` _staticmesh) (`SceneComponent.K2_GetComponentRotation` _staticmesh) (`self.Item Sketch`)) false false))
    (:`then_1`
      (`SphereComponent.SetSphereRadius` (`self.interaction_icon_show_range`) (`self.inner Sphere Radius`) true)
      (`SceneComponent.K2_SetRelativeLocation` (`self.Interact_icon`) (`self.Icon Location`) false false))
    (:`then_2`
      (if (`self.Debugging?`)
        (`SceneComponent.SetVisibility` _interaction_icon_show_range true false)
        (else
          (`SceneComponent.SetVisibility` _interaction_icon_show_range false false))))))