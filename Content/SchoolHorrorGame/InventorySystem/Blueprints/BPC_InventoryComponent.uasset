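; Inventory component for the horror game that stores picked-up items in a fixed-size array and displays them through WB_Inventory.
; B opens the widget with cursor and UI-only input.
; Adding takes the first slot that is empty or can stack the same item within the per-slot limit, then destroys the actor.
; Removal decrements or deletes the entry, and both operations refresh the widget; a separate function sets an Unlock flag.
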(event `self.ReceiveBeginPlay`
  ;[1 0.1722 0.9854 0.5] in play
  (bind _returnvalue (`|CreateWidget` "/Game/SchoolHorrorGame/InventorySystem/Widgets/WB_Inventory.WB_Inventory_C"))
  (set `self.Inventory Reference` _returnvalue)
  (`KismetArrayLibrary.Array_Resize` (`self.Items`) (`self.InventorySize`))
  (`/Game/SchoolHorrorGame/InventorySystem/Widgets/WB_Inventory.Refresh Inventory` (`self.Inventory Reference`) self))

(event `Key|B`
  (params (Key :type "Key Structure"))
  (bind _returnvalue (`GameplayStatics.GetPlayerController` 0))
  (bind _inventory_reference (`self.Inventory Reference`))
  (bind _inventory_reference_2 (`self.Inventory Reference`))
  ;[0.15 0.0311 0.08406 0.5] Opening
  (:`Pressed`
    (if (not (`Widget.IsInViewport` _inventory_reference))
      (`UserWidget.AddToViewport` _inventory_reference 0)
      (set `PlayerController.bShowMouseCursor` true _returnvalue)
      (`WidgetBlueprintLibrary.SetInputMode_UIOnlyEx` _returnvalue _inventory_reference_2)
      (set `UserWidget.bIsFocusable` true _inventory_reference_2))))

(fn `Add To Inventory`
  (params (Actor :type "/Game/SchoolHorrorGame/InventorySystem/Blueprints/BP_Item Object Reference"))
  (locals (NewLocalVar :type "/Game/SchoolHorrorGame/InventorySystem/Blueprints/BP_Item Object Reference"))
  (bind _currentindex (`self.CurrentIndex`))
  (bind _items (`self.Items`))
  (bind (_itemname _itemstackable_ _itemamount _itemimage _itemmesh _iteminventory_ _itemdescription _iteminspectionrotation _iteminspectionscale _itemcanues) (break `/Game/SchoolHorrorGame/InventorySystem/Blueprints/S_ItemStructure` (`/Game/SchoolHorrorGame/InventorySystem/Blueprints/BP_Item.Item` (`local.NewLocalVar`))))
  (set `local.NewLocalVar` Actor)
  (for (_array_element _array_index) (`self.Items`)
    (`/Engine/EditorBlueprintResources/StandardMacros.IsValid` Actor
      (:`Is Valid`
        (set `self.CurrentIndex` _array_index)
        (bind (_can_add_ _new_item_amount) (`self.Should Stack Items?` _array_element (`/Game/SchoolHorrorGame/InventorySystem/Blueprints/BP_Item.Item` (`local.NewLocalVar`))))
        (if _can_add_
          (set `self.newItemAmount` _new_item_amount)
          (`KismetArrayLibrary.Array_Set` (`self.Items`) (`self.CurrentIndex`) (make `/Game/SchoolHorrorGame/InventorySystem/Blueprints/S_ItemStructure` _itemname _itemstackable_ (`self.newItemAmount`) _itemimage _itemmesh _iteminventory_ _itemdescription _iteminspectionrotation _iteminspectionscale _itemcanues))
          (`/Game/SchoolHorrorGame/InventorySystem/Widgets/WB_Inventory.Refresh Inventory` (`self.Inventory Reference`) self :!label _label)
          (`Actor.K2_DestroyActor` (`local.NewLocalVar`))
          (return)
          (else
            (bind _has_space (`self.Space In Inventory?` _new_item_amount))
            (if _has_space
              (`KismetArrayLibrary.Array_Insert` _items (`/Game/SchoolHorrorGame/InventorySystem/Blueprints/BP_Item.Item` (`local.NewLocalVar`)) _currentindex)
              (`KismetArrayLibrary.Array_Remove` _items (- (`self.InventorySize`) _currentindex))
              (goto _label))))))))

(fn `are_Unlock`
  (`KismetSystemLibrary.PrintString` "are_Unlock")
  (set `self.Unlock` true))

(fn `Remove From Invenet`
  (params (`Item to Delete` :type "/Game/SchoolHorrorGame/InventorySystem/Blueprints/S_ItemStructure Structure"))
  (bind _items (`self.Items`))
  (bind (_itemname _itemstackable_ _itemamount _itemimage _itemmesh _iteminventory_ _itemdescription _iteminspectionrotation _iteminspectionscale _itemcanues) (break `/Game/SchoolHorrorGame/InventorySystem/Blueprints/S_ItemStructure` (`local.Item to Delete`)))
  (if (> (`.ItemAmount_26_8E7A754849E70FFBAAAAE2B65B35DBAE` (break `/Game/SchoolHorrorGame/InventorySystem/Blueprints/S_ItemStructure` `Item to Delete`)) 1)
    (`KismetArrayLibrary.Array_Set` (`self.Items`) (`KismetArrayLibrary.Array_Find` (`self.Items`) (`local.Item to Delete`)) (make `/Game/SchoolHorrorGame/InventorySystem/Blueprints/S_ItemStructure` _itemname _itemstackable_ (- _itemamount 1) _itemimage _itemmesh _iteminventory_ _itemdescription _iteminspectionrotation _iteminspectionscale _itemcanues))
    (else
      (`KismetArrayLibrary.Array_Remove` _items (`KismetArrayLibrary.Array_Find` (`self.Items`) (`local.Item to Delete`)))
      (`KismetArrayLibrary.Array_Resize` _items (`self.InventorySize`))))
  (`/Game/SchoolHorrorGame/InventorySystem/Widgets/WB_Inventory.Refresh Inventory` (`self.Inventory Reference`) self))

(fn `Should Stack Items?`
  (params (`Item From The Inventory` :type "/Game/SchoolHorrorGame/InventorySystem/Blueprints/S_ItemStructure Structure") (`Item From The Current Actor` :type "/Game/SchoolHorrorGame/InventorySystem/Blueprints/S_ItemStructure Structure"))
  (returns (`Can Add?` :type Boolean) (`New Item Amount` :type Integer))
  (bind (_itemname _itemstackable_ _itemamount) (break `/Game/SchoolHorrorGame/InventorySystem/Blueprints/S_ItemStructure` `Item From The Inventory`))
  (bind (_itemname_2 _itemstackable__2 _itemamount_2 _itemimage _itemmesh _iteminventory_) (break `/Game/SchoolHorrorGame/InventorySystem/Blueprints/S_ItemStructure` `Item From The Current Actor`))
  (bind _returnvalue (+ _itemamount _itemamount_2))
  (if (and _itemstackable__2 (`KismetTextLibrary.EqualEqual_TextText` _itemname _itemname_2) (<= _returnvalue (`self.MaxAmountPerItem`)) _iteminventory_)
    (return true _returnvalue)
    (else
      (return false _itemamount))))

(fn `Space In Inventory?`
  (params (`Item Amount From Inventory` :type Integer))
  (returns (`Has Space` :type Boolean))
  (if (== `Item Amount From Inventory` 0)
    (return true)
    (else
      (return false))))