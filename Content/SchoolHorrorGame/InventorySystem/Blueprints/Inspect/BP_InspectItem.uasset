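; Actor that presents an inventory item for close-up 3D inspection, viewed through a SceneCapture2D, with a W_Inspect widget showing its name and description.
; Inspect sets the mesh and moves input from the character to this actor; separate events set initial rotation and scale.
; Left-drag rotates the item, the wheel zooms via clamped capture FOV, and right-click resets both.
; E restores character input, removes the widget and destroys the actor.
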(event `/Game/SchoolHorrorGame/InventorySystem/Blueprints/interactinterface.Inspect`
  (params (Character :type "/Game/SchoolHorrorGame/Blueprints/BP_Player_Character Object Reference") (`Inspected Item` :type "StaticMesh Object Reference") (`Item Name` :type Text) (`Item Description` :type Text))
  (bind _returnvalue (`GameplayStatics.GetPlayerController` 0))
  (set `self.Character` Character)
  (`StaticMeshComponent.SetStaticMesh` (`self.Item`) `Inspected Item`)
  (bind _returnvalue_2 (`|CreateWidget` "/Game/SchoolHorrorGame/InventorySystem/Blueprints/Inspect/W_Inspect.W_Inspect_C" null `Item Name` `Item Description`))
  (bind _output_get (set `self.Inspect Widget Reference` _returnvalue_2))
  (`UserWidget.AddToViewport` _output_get 0)
  (`self.DisableInput` (`self.Character`) _returnvalue)
  (`self.EnableInput` _returnvalue))

(event `Key|E`
  (params (Key :type "Key Structure"))
  (bind _returnvalue (`GameplayStatics.GetPlayerController` 0))
  (bind _inspect_widget_reference (`self.Inspect Widget Reference`))
  (:`Pressed`
    (`self.DisableInput` _returnvalue)
    (`self.EnableInput` (`self.Character`) _returnvalue)
    (`/Engine/EditorBlueprintResources/StandardMacros.IsValid` _inspect_widget_reference
      (:`Is Valid`
        (`Widget.RemoveFromParent` _inspect_widget_reference)
        (set `self.Inspect Widget Reference` null)
        (`self.K2_DestroyActor`)))))

(event `Key|MouseScrollUp`
  (params (Key :type "Key Structure"))
  (bind _scenecapturecomponent2d (`self.SceneCaptureComponent2D`))
  ; Zoom in
  (:`Pressed`
    (set `SceneCaptureComponent2D.FOVAngle` (`KismetMathLibrary.FClamp` (- (`SceneCaptureComponent2D.FOVAngle` _scenecapturecomponent2d) 1.0) 30.0 80.0) _scenecapturecomponent2d)))

(event `Set Inspect rotation`
  (params (`Item rotation` :type "Rotator Structure"))
  (bind _item (`self.Item`))
  (bind (_returnvalue_location _returnvalue_rotation _returnvalue_scale) (`KismetMathLibrary.BreakTransform` (`SceneComponent.K2_GetComponentToWorld` _item)))
  ; Set Inspection Rotation
  (bind _output_get (set `self.Initial Rotation` `Item rotation`))
  (`SceneComponent.K2_SetWorldTransform` _item (`KismetMathLibrary.MakeTransform` _returnvalue_location _output_get _returnvalue_scale) false false))

(event `Key|MouseScrollDown`
  (params (Key :type "Key Structure"))
  (bind _scenecapturecomponent2d (`self.SceneCaptureComponent2D`))
  ; zoom out
  (:`Pressed`
    (set `SceneCaptureComponent2D.FOVAngle` (`KismetMathLibrary.FClamp` (+ (`SceneCaptureComponent2D.FOVAngle` _scenecapturecomponent2d) 1.0) 30.0 80.0) _scenecapturecomponent2d)))

(event `Set Inspect Scale`
  (params (`Inspection Scale` :type "Vector Structure"))
  (bind _item (`self.Item`))
  (bind (_returnvalue_location _returnvalue_rotation) (`KismetMathLibrary.BreakTransform` (`SceneComponent.K2_GetComponentToWorld` _item)))
  ; Set Inspect Scale
  (`SceneComponent.K2_SetWorldTransform` _item (`KismetMathLibrary.MakeTransform` _returnvalue_location _returnvalue_rotation `Inspection Scale`) false false))

(event `Key|LeftMouseButton`
  (params (Key :type "Key Structure"))
  ; Mouse
  (:`Pressed`
    (set `self.Rotate?` true))
  (:`Released`
    (set `self.Rotate?` false)))

(event `Key|RightMouseButton`
  (params (Key :type "Key Structure"))
  ; Mouse
  (:`Pressed`
    (`SceneComponent.K2_SetWorldRotation` (`self.Item`) (`self.Initial Rotation`) false false)
    (set `SceneCaptureComponent2D.FOVAngle` 50.0 (`self.SceneCaptureComponent2D`))))

(event `InputAxisKey|MouseY`
  (params (AxisValue :type "Float (single-precision)"))
  ; Mouse
  (if (`self.Rotate?`)
    (`SceneComponent.K2_SetWorldRotation` (`self.Item`) (`KismetMathLibrary.ComposeRotators` (`SceneComponent.K2_GetComponentRotation` (`self.Item`)) (`KismetMathLibrary.MakeRotator` 0.0 (* AxisValue -3.0))) false false)))

(event `InputAxisKey|MouseX`
  (params (AxisValue :type "Float (single-precision)"))
  ; Mouse
  (if (`self.Rotate?`)
    (`SceneComponent.K2_SetWorldRotation` (`self.Item`) (`KismetMathLibrary.ComposeRotators` (`SceneComponent.K2_GetComponentRotation` (`self.Item`)) (`KismetMathLibrary.MakeRotator` 0.0 0.0 (* AxisValue -3.0))) false false)))

(fn `UserConstructionScript`)