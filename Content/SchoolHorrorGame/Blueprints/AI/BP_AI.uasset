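; BP_AI is an enemy AI pawn that detects, chases and melees the player.
; Pawn sensing of a player-tagged pawn or any noise sets the "seeingPlayer" blackboard key and fades in chase violins.
; A looping timer clears that key, fading the music out if detection hasn't renewed it after a delay.
; AttackPlayer plays a guarded montage, applying damage via a forward sphere trace as it starts.
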(event `self.ReceiveBeginPlay`
  (`KismetSystemLibrary.K2_SetTimerDelegate` (delegate `Stop Scene Player`) 0.8 true))

(event `Stop Scene Player`
  (`BlackboardComponent.SetValueAsBool` (`AIBlueprintHelperLibrary.GetBlackboard` (`AIBlueprintHelperLibrary.GetAIController` self)) "seeingPlayer" false)
  (`KismetSystemLibrary.Delay` 1.0)
  (if (not (`BlackboardComponent.GetValueAsBool` (`AIBlueprintHelperLibrary.GetBlackboard` (`AIBlueprintHelperLibrary.GetAIController` self)) "seeingPlayer"))
    (bind _chasing_music (`self.chasing music`)
      (:`then`
        (`AudioComponent.FadeOut` _chasing_music 3.0 0.0 "Linear"))
      (:`else`))))

(event `self.PawnSensing.OnHearNoise`
  (params (Instigator :type "Pawn Object Reference") (Location :type "Vector Structure (by ref)") (Volume :type "Float (single-precision)"))
  (`BlackboardComponent.SetValueAsBool` (`AIBlueprintHelperLibrary.GetBlackboard` (`AIBlueprintHelperLibrary.GetAIController` self)) "seeingPlayer" true :!label _label)
  (`self.chasing music`
    (:`then`)
    (:`else`
      (bind _returnvalue (`GameplayStatics.SpawnSound2D` "/Game/StarterContent/Audio/ChasingViolins.ChasingViolins" 2.0 1.0 0.0 null))
      (bind _output_get (set `self.chasing music` _returnvalue))
      (`AudioComponent.FadeIn` _output_get 3.0 1.0 0.0 "Linear"))))

(event `self.PawnSensing.OnSeePawn`
  (params (Pawn :type "Pawn Object Reference"))
  (if (`self.ActorHasTag` Pawn "Player")
    (goto _label)))

(event `Attack Player`
  (bind _attack_trace_point (`self.Attack Trace point`))
  (bind _returnvalue (`SceneComponent.K2_GetComponentLocation` _attack_trace_point))
  (if (not (`self.attacking`))
    (set `self.attacking` true)
    (`|PlayMontage` (`self.Mesh`) "/Game/Characters/Mannequins/Anims/Pistol/NewAnimMontage.NewAnimMontage" 1.0 0.0 "None" false
      (:`then`
        (bind (_outhit _returnvalue_2) (`KismetSystemLibrary.SphereTraceSingleForObjects` _returnvalue (+ _returnvalue (* (`KismetMathLibrary.GetForwardVector` (`SceneComponent.K2_GetComponentRotation` _attack_trace_point)) 70.0)) 25.0 (`|MakeArray` "ObjectTypeQuery3" :!type "EObjectTypeQuery Enum")))
        (if _returnvalue_2
          (`GameplayStatics.ApplyDamage` (`.HitActor` (`GameplayStatics.BreakHitResult` _outhit)) 10.0)))
      (:`OnCompleted`
        (set `self.attacking` false)))))

(fn `UserConstructionScript`)