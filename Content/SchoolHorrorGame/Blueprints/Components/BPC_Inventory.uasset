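; BPC_Inventory is an inventory component for the horror game, with its item-adding logic only stubbed out.
; On BeginPlay it caches the player character as BP_Player_Character.
; AddToInventory loops while an amount remains and the inventory is not full, calling FindExistingSlot with "None" rather than the given ItemID.
; FindExistingSlot is empty, and the loop never updates the remaining amount or stores anything.
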(event `self.ReceiveBeginPlay`
  (bind _asbp_player_character (cast `/Game/SchoolHorrorGame/Blueprints/BP_Player_Character` (`GameplayStatics.GetPlayerCharacter` 0)))
  (set `self.Player_Ref` _asbp_player_character))

(fn `Add_to_inventory`
  (params (Item_ID :type Name) (Amount :type Integer))
  (locals (Amount_Remaining :type Integer) (Inventory_Full :type Boolean))
  (`|ExecutionSequence`
    (:`then_0`
      (bind _output_get (set `local.Amount_Remaining` Amount))
      (while (and (> _output_get 0) (not (`local.Inventory_Full`)))
        (`self.Find_existing_slot` "None")))))

(fn `Find_existing_slot`
  (params (Item_ID :type Name)))