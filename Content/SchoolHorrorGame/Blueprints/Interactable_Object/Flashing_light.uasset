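; Interactable spotlight actor for the school horror game that switches on and off when triggered.
; Activate and Deactivate share the same logic: each flips the LightOn flag and calls LightSwitch, so both act as toggles.
; Light_Switch sets the SpotLight visibility from that flag, and the construction script also calls LightSwitch to apply the initial state.
; Despite the Flashing_light name, no timer or automatic flicker is present.
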(event `self.Activate`
  (if (`self.Light_on`) :!label _label
    (set `self.Light_on` false)
    (else
      (set `self.Light_on` true)))
  (`self.Light_Switch`))

(event `self.Deactivate`
  (goto _label))

(event `Light_Switch`
  (bind _spotlight (`self.SpotLight`))
  (if (`self.Light_on`)
    (`SceneComponent.SetVisibility` _spotlight true false)
    (else
      (`SceneComponent.SetVisibility` _spotlight false false))))

(fn `UserConstructionScript`
  (`self.Light_Switch`))