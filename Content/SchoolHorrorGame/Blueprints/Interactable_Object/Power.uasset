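; Interactable power switch that toggles a set of target actors on and off when used.
; Interact locks further use and plays or reverses a timeline that tilts the switch button.
; When the timeline finishes, it sends activate or deactivate messages to every target actor and unlocks interaction.
; An overlap volume shows the widget interaction icon to the player, SetFoucs updates its focus, and GetDetails reports availability and prompt text.
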(event `self.ReceiveBeginPlay`
  (`self.Beginplay_Get_Refs`))

(event `self.Interact`
  (set `self.Can_intertact_variable` false)
  (`self.Switch`))

(event `Switch`
  (if (not (`self.Switch_on`))
    (bind (_direction _lightswitch) (`Timeline|Switch_Timeline` :!label _label)
      (:`Update`
        (`SceneComponent.K2_SetRelativeRotation` (`self.Light_Switch_button`) (`KismetMathLibrary.MakeRotator` 0.0 (`KismetMathLibrary.Lerp` 0.0 20.0 _lightswitch)) false false))
      (:`Finished`
        (switch `ETimelineDirection` _direction
          (:`Forward`
            (`self.Activate`))
          (:`Backward`
            (`self.Deactivate`)))))
    (else
      (goto _label :!via `Reverse`))))

(event `Activate`
  (for _array_element (`self.Target_Actors`)
    (message `/Game/SchoolHorrorGame/Blueprints/Interfaces/Electricity.Activate` _array_element))
  (set `self.Switch_on` true)
  (set `self.Can_intertact_variable` true))

(event `Deactivate`
  (for _array_element (`self.Target_Actors`)
    (message `/Game/SchoolHorrorGame/Blueprints/Interfaces/Electricity.Deactivate` _array_element))
  (set `self.Switch_on` false)
  (set `self.Can_intertact_variable` true))

(event `self.interaction_icon_show_collision.OnComponentBeginOverlap`
  (params (OverlappedComponent :type "PrimitiveComponent Object Reference") (OtherActor :type "Actor Object Reference") (OtherComp :type "PrimitiveComponent Object Reference") (OtherBodyIndex :type Integer) (bFromSweep :type Boolean) (SweepResult :type "HitResult Structure (by ref)"))
  (if (== OtherActor (`GameplayStatics.GetPlayerCharacter` 0))
    (`/Game/SchoolHorrorGame/Blueprints/UI/W_Interaction_icon.Show/Hide Interact Icon` (`self.Interact_icon_widget_Ref`) true)))

(event `self.interaction_icon_show_collision.OnComponentEndOverlap`
  (params (OverlappedComponent :type "PrimitiveComponent Object Reference") (OtherActor :type "Actor Object Reference") (OtherComp :type "PrimitiveComponent Object Reference") (OtherBodyIndex :type Integer))
  (if (== (`GameplayStatics.GetPlayerCharacter` 0) OtherActor)
    (`/Game/SchoolHorrorGame/Blueprints/UI/W_Interaction_icon.Show/Hide Interact Icon` (`self.Interact_icon_widget_Ref`) false)))

(event `self.Set_foucs`
  (params (Focus :type Boolean))
  (`/Game/SchoolHorrorGame/Blueprints/UI/W_Interaction_icon.Set_Focus` (`self.Interact_icon_widget_Ref`) Focus))

(fn `Beginplay_Get_Refs`
  (bind _asw_interaction_icon (cast `/Game/SchoolHorrorGame/Blueprints/UI/W_Interaction_icon` (`WidgetComponent.GetWidget` (`self.Interact_icon`))))
  (set `self.Interact_icon_widget_Ref` _asw_interaction_icon))

(fn `Get_Details`
  (returns (Result :type Boolean) (`Interaction text` :type Text))
  (return (`self.Can_intertact_variable`) (`self.Interaction Text`)))

(fn `UserConstructionScript`)