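; Gate door interactable that appears or disappears by toggling a Cylinder component, judging by its name serving as a barrier.
; Activate and Deactivate share the same logic, so either one flips the LightOn flag rather than setting a fixed state.
; A light-switch routine then sets the cylinder's visibility and collision from that flag.
; The construction script runs the same routine to apply the initial state.
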(event `self.Activate`
  (if (`self.Light_on`) :!label _label
    (set `self.Light_on` false)
    (else
      (set `self.Light_on` true)))
  (`self.Light_Switch`))

(event `self.Deactivate`
  (goto _label))

(event `Light_Switch`
  (if (`self.Light_on`)
    (`SceneComponent.SetVisibility` (`self.Cylinder`) true false)
    (`PrimitiveComponent.SetCollisionEnabled` (`self.Cylinder`) "QueryAndPhysics")
    (else
      (`SceneComponent.SetVisibility` (`self.Cylinder`) false false)
      (`PrimitiveComponent.SetCollisionEnabled` (`self.Cylinder`) "NoCollision"))))

(fn `UserConstructionScript`
  (`self.Light_Switch`))