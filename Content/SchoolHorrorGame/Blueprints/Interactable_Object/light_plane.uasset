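; Interactable light fixture Blueprint for the school horror game that switches the glow of its Cylinder mesh on and off.
; The construction script creates a dynamic material instance on the mesh and applies the current LightOn state.
; Activate and Deactivate share the same logic, so both toggle LightOn rather than forcing a state, then refresh the light.
; The refresh drives only the material's Emissive scalar parameter.
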(event `self.Activate`
  (if (`self.Light_on`) :!label _label
    (set `self.Light_on` false)
    (else
      (set `self.Light_on` true)))
  (`self.Light_Switch`))

(event `self.Deactivate`
  (goto _label))

(event `Light_Switch`
  (bind _emissive_material_ref (`self.Emissive_Material_Ref`))
  (if (`self.Light_on`)
    (`MaterialInstanceDynamic.SetScalarParameterValue` _emissive_material_ref "Emissive" 1.0)
    (else
      (`MaterialInstanceDynamic.SetScalarParameterValue` _emissive_material_ref "Emissive" 0.0))))

(fn `UserConstructionScript`
  (bind _cylinder (`self.Cylinder`))
  (bind _returnvalue (`PrimitiveComponent.CreateDynamicMaterialInstance` _cylinder 0 (`PrimitiveComponent.GetMaterial` _cylinder 0) "None"))
  (set `self.Emissive_Material_Ref` _returnvalue)
  (`self.Light_Switch`))