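; BP_objective is a placeable trigger volume that shows an objective message when the player walks in.
; It creates a WB_objective widget at BeginPlay, and the construction script sizes the box from ObjectiveBoxSize.
; The player's first overlap passes a DoOnce, sets the text, plays a sound and animates the widget in.
; After Duration, the animation plays in reverse; the widget is never removed from the viewport.
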(event `self.ReceiveBeginPlay`
  (bind _returnvalue (`|CreateWidget` "/Game/SchoolHorrorGame/Blueprints/UI/WB_objective.WB_objective_C" null (`self.objective Title Text`)))
  (set `self.WB Objective widget Ref` _returnvalue))

(event `self.objective Box.OnComponentBeginOverlap`
  (params (OverlappedComponent :type "PrimitiveComponent Object Reference") (OtherActor :type "Actor Object Reference") (OtherComp :type "PrimitiveComponent Object Reference") (OtherBodyIndex :type Integer) (bFromSweep :type Boolean) (SweepResult :type "HitResult Structure (by ref)"))
  (bind _wb_objective_widget_ref (`self.WB Objective widget Ref`))
  (bind _newanimation (`/Game/SchoolHorrorGame/Blueprints/UI/WB_objective.NewAnimation` _wb_objective_widget_ref))
  (if (== OtherActor (`GameplayStatics.GetPlayerCharacter` 0))
    (`/Engine/EditorBlueprintResources/StandardMacros.DoOnce` false
      (:`Completed`
        (set `/Game/SchoolHorrorGame/Blueprints/UI/WB_objective.objectiveText` (`self.objective Title Text`) (`self.WB Objective widget Ref`))
        (`GameplayStatics.PlaySound2D` (`self.Sound`) 1.0 1.0 0.0 null null)
        (`UserWidget.AddToViewport` _wb_objective_widget_ref 0)
        (`UserWidget.PlayAnimation` _wb_objective_widget_ref _newanimation 0.0 1 "Forward" 1.0 false)
        (`KismetSystemLibrary.Delay` (`self.Duration`))
        (`UserWidget.PlayAnimation` _wb_objective_widget_ref _newanimation 0.0 1 "Reverse" 1.0 false)))))

(fn `UserConstructionScript`
  (`BoxComponent.SetBoxExtent` (`self.objective Box`) (`self.objective Box Size`) true))